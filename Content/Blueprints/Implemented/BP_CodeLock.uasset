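; BP_CodeLock is an interactable code lock that stays unusable until all its number keys are found, then unlocks its linked drawers or doors.
; SetNumberKey flags entries in a boolean array, enabling the lock when all are true, otherwise printing a decremented count of numbers still needed.
; Interaction toggles the lock menu through BP_HUD_Core once enabled, or prints a placeholder message.
; CodeIsValid lets every referenced drawer/door open, then destroys the lock.
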(event `self.ReceiveBeginPlay`
  ;[0.05 0.05 0.05] Init Array Lenght
  (set `self.ArrayLength` (`KismetArrayLibrary.Array_Length` (`self.BArrNumbersKey`))))

(event `/Game/Blueprints/Implemented/BPI_SetLock.Set Number Key`
  (params (Index :type Integer))
  (bind _barrnumberskey (`self.BArrNumbersKey`))
  ;[0.05 0.05 0.05] Check if lock can be use
  (`KismetArrayLibrary.Array_Set` _barrnumberskey Index true)
  (for _array_element _barrnumberskey
    (if _array_element
      (set `self.BIsArrayTrue` true)
      (else
        (set `self.BIsArrayTrue` false)
        (break))))
  (if (`self.BIsArrayTrue`)
    (set `self.BCanBeUsed` true)
    (`KismetSystemLibrary.PrintString` "I can use the lock now !")
    (else
      (bind _result (`/Engine/EditorBlueprintResources/StandardMacros.DecrementInt` (`self.ArrayLength`))
        (:`  `
          (`KismetSystemLibrary.PrintString` (`KismetStringLibrary.Concat_StrStr` "I still need " (`KismetStringLibrary.Conv_IntToString` _result) " numbers.") true true (struct :`G` 0.66 :`B` 1.0 :`A` 1.0) 5.0))))))

(event `/Game/Blueprints/Implemented/Player/BPI_Interaction.Interaction`
  (params (CameraVector :type "Vector Structure"))
  ;[0.05 0.05 0.05] Open Lock Widget
  (if (`self.BCanBeUsed`)
    (bind _asbp_hud_core (cast `/Game/Blueprints/Implemented/Widget/BP_HUD_Core` (`PlayerController.GetHUD` (`GameplayStatics.GetPlayerController` 0))))
    (`/Game/Blueprints/Implemented/Widget/BP_HUD_Core.Toggle_LockMenu` _asbp_hud_core)
    (else
      (`KismetSystemLibrary.PrintString` "It looks like a lock with a code ( j'avais pas de moddé donc on fait avec ce que l'on a )  \n:)" true true (struct :`G` 0.66 :`B` 1.0 :`A` 1.0) 5.0))))

(event `CodeIsValid`
  (for _array_element (`self.DrawerDoorRef`)
    (set `/Game/Blueprints/Implemented/BP_DrawerDoor.BCanOpen` true _array_element))
  (`self.K2_DestroyActor`))

(fn `UserConstructionScript`)