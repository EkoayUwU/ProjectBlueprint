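; BP_Key is a pickup that the player collects through an Interaction event, acting as either key one or key two.
; It sets the matching key flag on the first-person character, chosen by two boolean properties on the key.
; Key one also unlocks its referenced door directly by setting BCanOpen, while key two only sets the character flag.
; The actor destroys itself after the interaction.
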(event `/Game/Blueprints/Implemented/Player/BPI_Interaction.Interaction`
  (params (CameraVector :type "Vector Structure"))
  (`|ExecutionSequence`
    (:`then_0`
      (bind _asbp_first_person_character (cast `/Game/Blueprints/Implemented/Player/BP_FirstPersonCharacter` (`GameplayStatics.GetPlayerCharacter` 0)))
      (if (`self.BIsKeyOne`)
        (set `/Game/Blueprints/Implemented/Player/BP_FirstPersonCharacter.BKeyOne` true _asbp_first_person_character)
        (set `/Game/Blueprints/Implemented/BP_Door.BCanOpen` true (`self.DoorRef`))
        (elif (`self.BIsKeyTwo`)
          (set `/Game/Blueprints/Implemented/Player/BP_FirstPersonCharacter.BKeyTwo` true _asbp_first_person_character))))
    (:`then_1`
      (`self.K2_DestroyActor`))))

(fn `UserConstructionScript`)