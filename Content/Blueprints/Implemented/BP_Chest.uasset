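; Interactable chest that opens once the first-person player character holds both key flags.
; On interaction, a DoOnce starts a timeline that rolls the cover open along a curve, turns on a spotlight and clears the can-open flag.
; Disconnected leftover logic would attach two dummy key meshes to the cover and animate key rotation, but never runs.
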(event `/Game/Blueprints/Implemented/Player/BPI_Interaction.Interaction`
  (params (CameraVector :type "Vector Structure"))
  (if (`self.BCanBeOpen`)
    (bind _asbp_first_person_character (cast `/Game/Blueprints/Implemented/Player/BP_FirstPersonCharacter` (`GameplayStatics.GetPlayerCharacter` 0)))
    (if (and (`/Game/Blueprints/Implemented/Player/BP_FirstPersonCharacter.BKeyOne` _asbp_first_person_character) (`/Game/Blueprints/Implemented/Player/BP_FirstPersonCharacter.BKeyTwo` _asbp_first_person_character))
      (`/Engine/EditorBlueprintResources/StandardMacros.DoOnce` false
        (:`Completed`
          (bind (_direction _chestopeningcurve) (`Timeline|Timeline`)
            (:`Update`
              (`SceneComponent.K2_SetRelativeRotation` (`self.Chest_cover6_StaticMeshComponent0`) (`KismetMathLibrary.MakeRotator` (* (`self.RotationAngle`) _chestopeningcurve)) false false)
              (`|ExecutionSequence`
                (:`then_0`
                  (`SceneComponent.SetVisibility` (`self.SpotLight`) true false))
                (:`then_1`
                  (set `self.BCanBeOpen` false))))))))))

(fn `UserConstructionScript`)