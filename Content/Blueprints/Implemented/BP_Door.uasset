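; BP_Door is an interactable double door that swings open and closed, or prints a key-required message when opening is not allowed.
; On interaction while closed, it compares the camera vector to the aperture's right vector to set the swing direction.
; A FlipFlop plays or reverses a timeline that rotates both leaves in opposite yaw directions.
; An opening flag ignores interactions during movement.
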(event `/Game/Blueprints/Implemented/Player/BPI_Interaction.Interaction`
  (params (CameraVector :type "Vector Structure"))
  (bind _returnvalue (`KismetMathLibrary.Abs` (`self.RotationAngle`)))
  (if (`self.BCanOpen`)
    (if (not (`self.BIsOpening`))
      (if (`self.BIsDoorOpen`)
        _
        (elif (== CameraVector (`SceneComponent.GetRightVector` (`self.Door_aperture_2_StaticMeshComponent0`)) :`ErrorTolerance` 1.0)
          (set `self.RotationAngle` (* _returnvalue -1.0))
          (else
            (set `self.RotationAngle` _returnvalue))))
      (`/Engine/EditorBlueprintResources/StandardMacros.FlipFlop`
        (:`A`
          (set `self.BIsDoorOpen` true)
          (set `self.BIsOpening` true)
          (bind (_direction _newtrack) (`Timeline|Door_Movement` :!label _label)
            (:`Update`
              (bind _returnvalue_2 (* _newtrack (`self.RotationAngle`)))
              (`SceneComponent.K2_SetRelativeRotation` (`self.Door_3_StaticMeshLeft`) (`KismetMathLibrary.MakeRotator` 0.0 0.0 (* _returnvalue_2 -1.0)) false false)
              (`SceneComponent.K2_SetRelativeRotation` (`self.Door_4_StaticMeshRight`) (`KismetMathLibrary.MakeRotator` 0.0 0.0 _returnvalue_2) false false))
            (:`Finished`
              (set `self.BIsOpening` false))))
        (:`B`
          (set `self.BIsDoorOpen` false)
          (set `self.BIsOpening` true)
          (goto _label :!via `Reverse`))))
    (else
      (`KismetSystemLibrary.PrintString` "You need a Key"))))

(fn `UserConstructionScript`)