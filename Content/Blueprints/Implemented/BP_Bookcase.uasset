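; BP_Bookcase is a bookcase that slides horizontally to a target location when its EventMove event fires.
; The event plays a world camera shake at the bookcase, records its starting location, then runs the Movement timeline.
; A vector track supplies separate X and Y alphas to interpolate SharedRoot toward TargetLocation, while Z stays at its starting height.
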(event `EventMove`
  (bind (_initiallocation_x _initiallocation_y _initiallocation_z) (`KismetMathLibrary.BreakVector` (`self.InitialLocation`)))
  (bind (_targetlocation_x _targetlocation_y) (`KismetMathLibrary.BreakVector` (`self.TargetLocation`)))
  (`GameplayStatics.PlayWorldCameraShake` "/Game/Blueprints/Implemented/Player/BP_CameraShake.BP_CameraShake_C" (`SceneComponent.K2_GetComponentLocation` (`self.SharedRoot`)) 0.0 500.0)
  (set `self.InitialLocation` (`SceneComponent.K2_GetComponentLocation` (`self.SharedRoot`)))
  (bind (_direction _movementvalue) (`Timeline|Movement`)
    (:`Update`
      (`SceneComponent.K2_SetWorldLocation` (`self.SharedRoot`) (`KismetMathLibrary.MakeVector` (`KismetMathLibrary.Lerp` _initiallocation_x _targetlocation_x (.x _movementvalue)) (`KismetMathLibrary.Lerp` _initiallocation_y _targetlocation_y (.y _movementvalue)) _initiallocation_z) false false))))

(fn `UserConstructionScript`)